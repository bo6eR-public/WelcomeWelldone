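; Weapon equipment instance that updates the owning character's animation when a weapon is equipped or unequipped.
; A LinkAnimLayers event links the supplied anim layer class to the character mesh, falling back to a default layer when that class is invalid.
; It then plays the equip or unequip montage on the same mesh, chosen by the IsEquipped state.
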(event EventLinkAnimLayers
  (params (LinkedInstance :type Anim%20Instance%20Class%20Reference))
  (bind _returnvalue (Class|WellEquipmentInstance|GetOwnerasCharacter))
  (bind _mesh (Variables|/Script/Engine.Character|GetMesh _returnvalue))
  (bind _returnvalue_2 (Utilities|SelectSuitableLayer LinkedInstance (Variables|Default|GetDefaultAnimLayer))
    (:Out
      (Components|SkeletalMesh|AnimationBlueprintLinking|LinkAnimClassLayers _mesh _returnvalue_2)
      (bind _returnvalue_3 (Utilities|SelectSuitableMontage)
        (:Out
          (Animation|Montage|PlayMontage _mesh _returnvalue_3))))))