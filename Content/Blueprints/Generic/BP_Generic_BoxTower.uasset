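; Generic box tower actor that procedurally stacks copies of one mesh into a vertical column.
; The construction script clears the TowerBoxes instanced mesh component, then adds TowerHeight local-space instances spaced by the mesh's bounding-box height.
; All boxes share one XY offset from Angle and Radius, and each gets a random yaw within a limited range.
; The event graph holds only disabled default events, so nothing runs during play.
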(event EventBeginPlay)

(event Collision|EventActorBeginOverlap
  (params (OtherActor :type Actor%20Object%20Reference)))

(event EventTick
  (params (DeltaSeconds :type Float%20%28single-precision%29)))

(fn ConstructionScript
  (bind _towerboxes (Variables|Default|GetTowerBoxes))
  (bind _angle (Variables|Default|GetAngle))
  (bind _radius (Variables|Default|GetRadius))
  (bind _staticmesh (Variables|/Script/Engine.StaticMeshComponent|GetStaticMesh _towerboxes))
  (bind _returnvalue (StaticMesh|GetBoundingBox _staticmesh))
  (Components|InstancedStaticMesh|ClearInstances (Variables|Default|GetTowerBoxes))
  (LocalVariables|SetBoxHeight (.Z (Math|Vector|BreakVector (- (.max _returnvalue) (.min _returnvalue)))))
  (for _index (range 0 (- (Variables|Default|GetTowerHeight) 1))
    (LocalVariables|SetBoxIndex _index)
    (Components|InstancedStaticMesh|AddInstance (Variables|Default|GetTowerBoxes) (Math|Transform|MakeTransform (Math|Vector|MakeVector (* (Math|Trig|Cos(Degrees) _angle) _radius) (* _radius (Math|Trig|Sin(Degrees) _angle)) (* (LocalVariables|GetBoxIndex) (LocalVariables|GetBoxHeight))) (CallFunction|MakeRandomBoxRotatiom)) false)))

(fn MakeRandomBoxRotatiom
  (return (Math|Rotator|MakeRotator 0.0 0.0 (Math|Random|RandomFloatinRange 0.0 45.0))))