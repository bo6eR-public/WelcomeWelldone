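; Generic parkour actor that builds a rising spiral of blocks as instances of the BlockMeshes component.
; The construction script, on authority only, places each block by stepping the angle around a radius and raising height per index.
; It appends each transform to CachedTransforms, whose OnRep clears and rebuilds the instances from that array so clients get the same layout.
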(fn ConstructionScript
  (bind _radius (Variables|Default|GetRadius))
  (Networking|SwitchHasAuthority
    (:Authority
      (Components|InstancedStaticMesh|ClearInstances (Variables|Default|GetBlockMeshes))
      (for _index (range 0 (- (Variables|Default|GetBlocksCount) 1))
        (LocalVariables|SetBlockIndex _index)
        (Components|InstancedStaticMesh|AddInstance (Variables|Default|GetBlockMeshes) (Math|Transform|MakeTransform (Math|Vector|MakeVector (* (Math|Trig|Cos(Radians) (Math|Trig|DegreesToRadians (* _index (Variables|Default|GetAngle%20Max)))) _radius) (* _radius (Math|Trig|Sin(Radians) (Math|Trig|DegreesToRadians (* _index (Variables|Default|GetAngle%20Max))))) (* (Variables|Default|GetHeightStep) (LocalVariables|GetBlockIndex))) (Math|Rotator|MakeRotator 0.0 0.0 0.0)) false)
        (Utilities|Array|Add (Variables|Default|GetCachedTransforms) (Math|Transform|MakeTransform (Math|Vector|MakeVector (* (Math|Trig|Cos(Radians) (Math|Trig|DegreesToRadians (* _index (Variables|Default|GetAngle%20Max)))) _radius) (* _radius (Math|Trig|Sin(Radians) (Math|Trig|DegreesToRadians (* _index (Variables|Default|GetAngle%20Max))))) (* (Variables|Default|GetHeightStep) (LocalVariables|GetBlockIndex))) (Math|Rotator|MakeRotator 0.0 0.0 0.0)))))))

(fn OnRepCachedTransforms
  (Components|InstancedStaticMesh|ClearInstances (Variables|Default|GetBlockMeshes))
  (for _index (range 0 (- (Variables|Default|GetBlocksCount) 1))
    (Components|InstancedStaticMesh|AddInstance (Variables|Default|GetBlockMeshes) (Utilities|Array|Get(acopy) (Variables|Default|GetCachedTransforms) _index) false)))