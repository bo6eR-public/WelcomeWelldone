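; BP_Generic_Benches is a generic actor that builds a straight row of repeated bench instances.
; The construction script clears the Benches instanced mesh component, then adds Count local-space instances along X, spaced by StepLenght with no rotation or scaling.
; The event graph holds only disabled placeholder events, so the actor has no runtime logic.
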(event EventBeginPlay)

(event Collision|EventActorBeginOverlap
  (params (OtherActor :type Actor%20Object%20Reference)))

(event EventTick
  (params (DeltaSeconds :type Float%20%28single-precision%29)))

(fn ConstructionScript
  (Components|InstancedStaticMesh|ClearInstances (Variables|Default|GetBenches))
  (for _index (range 0 (- (Variables|Default|GetCount) 1))
    (Components|InstancedStaticMesh|AddInstance (Variables|Default|GetBenches) (Math|Transform|MakeTransform (Math|Vector|MakeVector (* _index (Variables|Default|GetStepLenght)) 0.0 0.0)) false)))