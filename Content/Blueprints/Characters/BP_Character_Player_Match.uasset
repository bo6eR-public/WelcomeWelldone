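; Match player character Blueprint that handles networked cosmetic effects for gameplay modifiers and hit feedback.
; Each public event passes an authority check, then calls a multicast counterpart.
; Modifiers drive head scale through the anim instance, invisibility through translucent material swaps, and wallhack through custom depth on the target character's mesh.
; Hit feedback plays a 2D body-hit sound and spawns short-lived bullet decals aligned to the surface normal.
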(event Custom|SetNewMeshMaterial_Multicast
  (params (Target%20Actor :type Actor%20Object%20Reference) (Enabled%20Wallhack :type Boolean))
  ;[0.15 0.15 0.15 0.5] NetMulticast applying wallhack modifier
  (bind _ascharacter (Utilities|Casting|CastToCharacter Target%20Actor))
  (Rendering|SetRenderCustomDepth (Variables|/Script/Engine.Character|GetMesh _ascharacter) Enabled%20Wallhack))

(event Custom|SetNewHeadScale_Multicast
  (params (New%20Scale :type Vector))
  ;[0.15 0.15 0.15 0.5] NetMulticast applying enlarge head scale
  (bind _asabp_char_master (Utilities|Casting|CastToABP_Char_Master (Components|SkeletalMesh|GetAnimInstance (Variables|Character|GetMesh))))
  (Variables|/Game/Blueprints/Animation/ABP_Char_Master.ABP_Char_Master_C|SetHead%20Scale _asabp_char_master New%20Scale))

(event Custom|PlayHitSound_Multicast
  ;[0.15 0.15 0.15 0.5] NetMulticast playing body hit sound
  (Audio|PlaySound2D "/Game/External/Sounds/Character/Hitting/SC_BodyHit.SC_BodyHit" 1.0 1.0 0.0 0 0))

(event Custom|SpawnHitEffect_Multicast
  (params (Location :type Vector) (Normal :type Vector))
  ;[0.15 0.15 0.15 0.5] NetMulticast spawning bullet hit decal
  (bind _returnvalue (Rendering|Decal|SpawnDecalatLocation "/Game/External/Materials/Hit/MI_BulltetHit.MI_BulltetHit" "3.000000,6.000000,6.000000" Location (Math|Conversions|RotationFromXVector Normal) 5.0))
  (Utilities|IsValid _returnvalue
    (:Is%20Valid
      (Rendering|Components|Decal|SetFadeScreenSize _returnvalue 0.0))))

(event Custom|ApplyInvisibility_Multicast
  (params (bInvisibility :type Boolean))
  (bind _mesh (Variables|Character|GetMesh))
  (bind _mesh_2 (Variables|Character|GetMesh))
  (if bInvisibility
    (Rendering|Material|SetMaterial _mesh_2 0 "/Game/External/Materials/Character/MI_Translusent.MI_Translusent")
    (Rendering|Material|SetMaterial _mesh_2 1 "/Game/External/Materials/Character/MI_Translusent.MI_Translusent")
    (else
      (Rendering|Material|SetMaterial _mesh 0 "/Game/External/Materials/Character/MI_CellShading_Character_01.MI_CellShading_Character_01")
      (Rendering|Material|SetMaterial _mesh 1 "/Game/External/Materials/Character/MI_CellShading_Character_02.MI_CellShading_Character_02"))))

(event EventApplyEnlargeHeadModifier
  (params (NewScale :type Vector :default "0, 0, 0"))
  ;[0.15 0.15 0.15 0.5] NetMulticast applying enlarge head scale
  (Networking|SwitchHasAuthority
    (:Authority
      (CallFunction|SetNewHeadScaleMulticast NewScale))))

(event EventApplyWallhackModifier
  (params (Target%20Actor :type Actor%20Object%20Reference) (bEnabledWallhack :type Boolean))
  ;[0.15 0.15 0.15 0.5] NetMulticast applying wallhack modifier
  (Networking|SwitchHasAuthority
    (:Authority
      (CallFunction|SetNewMeshMaterialMulticast Target%20Actor bEnabledWallhack))))

(event EventSpawnHitEffect
  (params (Hit%20Location :type Vector :default "0, 0, 0") (Hit%20Normal :type Vector :default "0, 0, 0"))
  ;[0.15 0.15 0.15 0.5] NetMulticast spawning bullet hit decal
  (Networking|SwitchHasAuthority
    (:Authority
      (CallFunction|SpawnHitEffectMulticast Hit%20Location Hit%20Normal))))

(event EventPlayHitSound
  ;[0.15 0.15 0.15 0.5] NetMulticast playing body hit sound
  (Networking|SwitchHasAuthority
    (:Authority
      (CallFunction|PlayHitSoundMulticast))))

(event EventApplyInvisibilityModifier
  (params (bInvisible :type Boolean))
  (Networking|SwitchHasAuthority
    (:Authority
      (CallFunction|ApplyInvisibilityMulticast bInvisible))))

(fn ConstructionScript)